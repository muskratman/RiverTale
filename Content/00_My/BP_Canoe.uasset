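; Player canoe Blueprint that registers itself with BP_Player_Controller and drives an orbiting spring-arm camera.
; Look and scroll axes rotate and zoom the arm, and R saves the current view as default.
; When camera input stops, a DoOnce-gated three-second timer restores the default view; further movement cancels it.
; An unconnected timeline loop would rock the boat with random alternating roll relative to the river anchor, but never runs.
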(event Custom|Set_Camera_Rot_Loc
  ;[1 1 1] MOUSE & Camera
  (if (Math|Rotator|Equal(Rotator) (Variables|Default|GetCurr_Spring_Arm_Rot) (Variables|/Script/Engine.SceneComponent|GetRelativeRotation (Variables|Default|GetSpringArm)) 0.0001)
    (if (== (Variables|Default|GetCurr_Spring_Arm_Length) (Variables|/Script/Engine.SpringArmComponent|GetTargetArmLength (Variables|Default|GetSpringArm)))
      (Transformation|SetRelativeRotation (Variables|Default|GetSpringArm) (Variables|Default|GetDefault_Spring_Arm_Rot) false false)
      (Variables|/Script/Engine.SpringArmComponent|SetTargetArmLength (Variables|Default|GetSpringArm) (Variables|Default|GetDefault_Spring_Arm_Length)))))

(event EventBeginPlay
  (bind _springarm (Variables|Default|GetSpringArm))
  (bind _springarm_2 (Variables|Default|GetSpringArm))
  (Variables|Default|SetIsometric_View false)
  (bind _asbp_player_controller (Utilities|Casting|CastToBP_Player_Controller (Game|GetPlayerController 0))
    (:then
      (Variables|/Game/00_My/BP_Player_Controller.BP_Player_Controller_C|SetBP_Canoe _asbp_player_controller self))
    (:CastFailed
      (Development|PrintString "CAST FAILED   controller")))
  (Utilities|FlowControl|Sequence
    (:then_0
      (Variables|/Script/Engine.SpringArmComponent|SetTargetArmLength _springarm (Variables|Default|GetDefault_Spring_Arm_Length))
      (Transformation|SetRelativeRotation _springarm (Variables|Default|GetDefault_Spring_Arm_Rot) false false)
      (if (Variables|Default|GetIsometric_View)
        (Variables|/Script/Engine.SpringArmComponent|SetTargetArmLength _springarm_2 2.5e+03)
        (Transformation|SetRelativeRotation _springarm_2 "-35.000000,-30.000000, 0" false false)))))

(event Input|AxisEvents|InputAxisLookUp
  (params (AxisValue :type Float%20%28single-precision%29))
  ;[1 1 1] MOUSE & Camera
  (Transformation|AddRelativeRotation (Variables|Default|GetSpringArm) (Math|Rotator|MakeRotator 0.0 (* AxisValue 3.0) 0.0) false false)
  (if (Math|Rotator|Equal(Rotator) (Variables|Default|GetCurr_Spring_Arm_Rot) (Variables|/Script/Engine.SceneComponent|GetRelativeRotation (Variables|Default|GetSpringArm)) 0.2)
    (Utilities|FlowControl|DoOnce false :!label _label
      (:Completed
        (bind _returnvalue (Utilities|Time|SetTimerbyEvent (delegate Custom|Set_Camera_Rot_Loc) 3.0))))
    (else
      (Variables|Default|SetCurr_Spring_Arm_Rot (Variables|/Script/Engine.SceneComponent|GetRelativeRotation (Variables|Default|GetSpringArm)))
      (Utilities|Time|ClearandInvalidateTimerbyHandle _returnvalue)
      (Utilities|Time|PauseTimerbyHandle _returnvalue)
      (goto _label Reset))))

(event Input|AxisEvents|InputAxisLookRight
  (params (AxisValue :type Float%20%28single-precision%29))
  ;[1 1 1] MOUSE & Camera
  (Transformation|AddRelativeRotation (Variables|Default|GetSpringArm) (Math|Rotator|MakeRotator 0.0 0.0 (* AxisValue 3.0)) false false)
  (if (Math|Rotator|Equal(Rotator) (Variables|Default|GetCurr_Spring_Arm_Rot) (Variables|/Script/Engine.SceneComponent|GetRelativeRotation (Variables|Default|GetSpringArm)) 0.2)
    (Utilities|FlowControl|DoOnce false :!label _label
      (:Completed
        (bind _returnvalue (Utilities|Time|SetTimerbyEvent (delegate Custom|Set_Camera_Rot_Loc) 3.0))))
    (else
      (Variables|Default|SetCurr_Spring_Arm_Rot (Variables|/Script/Engine.SceneComponent|GetRelativeRotation (Variables|Default|GetSpringArm)))
      (Utilities|Time|ClearandInvalidateTimerbyHandle _returnvalue)
      (Utilities|Time|PauseTimerbyHandle _returnvalue)
      (goto _label Reset))))

(event Input|AxisEvents|InputAxisScroll_UP
  (params (AxisValue :type Float%20%28single-precision%29))
  (bind _springarm (Variables|Default|GetSpringArm))
  ;[1 1 1] MOUSE & Camera
  (Variables|/Script/Engine.SpringArmComponent|SetTargetArmLength _springarm (+ (* (Class|Actor|GetInputAxisKeyValue) 5e+01) (Variables|/Script/Engine.SpringArmComponent|GetTargetArmLength _springarm)))
  (if (== (Variables|Default|GetCurr_Spring_Arm_Length) (Variables|/Script/Engine.SpringArmComponent|GetTargetArmLength (Variables|Default|GetSpringArm)))
    (Utilities|FlowControl|DoOnce false :!label _label
      (:Completed
        (bind _returnvalue (Utilities|Time|SetTimerbyEvent (delegate Custom|Set_Camera_Rot_Loc) 3.0))))
    (else
      (Variables|Default|SetCurr_Spring_Arm_Length (Variables|/Script/Engine.SpringArmComponent|GetTargetArmLength (Variables|Default|GetSpringArm)))
      (Utilities|Time|ClearandInvalidateTimerbyHandle _returnvalue)
      (Utilities|Time|PauseTimerbyHandle _returnvalue)
      (goto _label Reset))))

(event Input|KeyboardEvents|R
  (params (Key :type Key%20Structure :default "None"))
  ;[1 1 1] MOUSE & Camera
  (:Pressed
    (Variables|Default|SetDefault_Spring_Arm_Rot (Variables|Default|GetCurr_Spring_Arm_Rot))
    (Variables|Default|SetDefault_Spring_Arm_Length (Variables|Default|GetCurr_Spring_Arm_Length))))

(fn ConstructionScript)