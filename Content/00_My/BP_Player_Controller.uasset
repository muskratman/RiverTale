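; Player controller that sidesteps a canoe left or right in fixed steps on MoveLeft and MoveRight input.
; Each press sets target location and yaw, then restarts separate move and rotation timelines, ignoring input while a side move plays.
; The timelines lerp the canoe's relative location and yaw, preserving its current pitch and roll.
; The finished move stores the new location as the next starting point.
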(event EventBeginPlay)

(event EventTick
  (params (DeltaSeconds :type Float%20%28single-precision%29)))

(event Input|ActionEvents|InputActionMoveRight
  (params (Key :type Key%20Structure :default "None"))
  (bind _canoe_loc_curr (Variables|Default|GetCanoe_Loc_Curr))
  (:Pressed
    (if (not (Audio|Components|Audio|IsPlaying (Variables|Default|GetTL_Side_Move)))
      (Development|PrintString "RIGHT")
      (Variables|Default|SetCanoe_Rot_Next "0.000000,-10.000000, 0")
      (Variables|Default|SetCanoe_Loc_Next (Math|Vector|MakeVector (.x _canoe_loc_curr) (+ (.y _canoe_loc_curr) -2e+02) (.z _canoe_loc_curr)))
      (Audio|Components|Audio|Stop (Variables|Default|GetTL_Rotation))
      (Components|Timeline|PlayfromStart (Variables|Default|GetTL_Side_Move))
      (Components|Timeline|PlayfromStart (Variables|Default|GetTL_Rotation)))))

(event Input|ActionEvents|InputActionMoveLeft
  (params (Key :type Key%20Structure :default "None"))
  (bind _canoe_loc_curr (Variables|Default|GetCanoe_Loc_Curr))
  (:Pressed
    (if (not (Audio|Components|Audio|IsPlaying (Variables|Default|GetTL_Side_Move)))
      (Development|PrintString "LEFT")
      (Variables|Default|SetCanoe_Rot_Next "0.000000,10.000000, 0")
      (Variables|Default|SetCanoe_Loc_Next (Math|Vector|MakeVector (.x _canoe_loc_curr) (+ (.y _canoe_loc_curr) 2e+02) (.z _canoe_loc_curr)))
      (Audio|Components|Audio|Stop (Variables|Default|GetTL_Rotation))
      (Components|Timeline|PlayfromStart (Variables|Default|GetTL_Side_Move))
      (Components|Timeline|PlayfromStart (Variables|Default|GetTL_Rotation)))))

(fn ConstructionScript)