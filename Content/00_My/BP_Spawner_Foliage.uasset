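; Spawner that scatters instanced trees, grass and rocks around a given location, in a box widened by river scale.
; Place_Foliage runs each category in turn through MacroSpawn, spreading passes over short delays; only tree count follows river scale.
; Each pass traces down from random points, rejecting points too close within that pass, and adds randomly yawed, scaled instances.
; A looping timer removes instances left behind the player along X.
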(event Custom|Place_Foliage
  (params (River_Scale :type Float%20%28single-precision%29) (Spawn_Loc :type Vector))
  (bind _returnvalue (/ River_Scale 2.0))
  (Variables|Default|SetSpawn_Location Spawn_Loc)
  (Variables|Default|SetContainer_Scale (Math|Vector|MakeVector 2.5e+03 (* River_Scale 2e+03) 2e+03))
  (Variables|Random|SetMin_Max_Num_Tree (* (Variables|Default|GetMin_Max_Num_Def_Tree) _returnvalue))
  (Variables|Random|SetMin_Max_Num_Grass (* (Variables|Default|GetMin_Max_Num_Def_Grass) _returnvalue))
  (Variables|Random|SetMin_Max_Num_Rocks (* (Variables|Default|GetMin_Max_Num_Def_Rocks) _returnvalue))
  (Components|Box|SetBoxExtent (Variables|Default|GetContainer) (Variables|Default|GetContainer_Scale) true)
  (Utilities|MacroSpawn (Variables|Random|GetMin_Max_Num_Tree) (Variables|Meshes|GetTree_Arr) (Variables|Default|GetInst_Mesh_Tree_Arr) (Variables|Random|GetBlock_Sphere_Tree) (Variables|Random|GetMin_Max_Scale_Tree)
    (:then_0
      (Utilities|MacroSpawn (Variables|Default|GetMin_Max_Num_Def_Grass) (Variables|Meshes|GetGrass_Arr) (Variables|Default|GetInst_Mesh_Grass_Arr) (Variables|Random|GetBlock_Sphere_Grass) (Variables|Random|GetMin_Max_Scale_Grass)
        (:then_0
          (Utilities|MacroSpawn (Variables|Default|GetMin_Max_Num_Def_Rocks) (Variables|Meshes|GetRocks_Arr) (Variables|Default|GetInst_Mesh_Rocks_Arr) (Variables|Random|GetBlock_Sphere_Rocks) (Variables|Random|GetMin_Max_Scale_Rocks)))))))

(event Custom|Remove_Instance_Timer
  (Variables|Default|SetCurr_Pawn_Location_X (.x (Transformation|GetActorLocation (Game|Player|GetPlayerPawn 0))))
  (CallFunction|FDestroyInstance (Variables|Default|GetInst_Mesh_Tree_Arr) 3e+03)
  (CallFunction|FDestroyInstance (Variables|Default|GetInst_Mesh_Grass_Arr) 3e+03)
  (CallFunction|FDestroyInstance (Variables|Default|GetInst_Mesh_Rocks_Arr) 3e+03))

(event EventBeginPlay
  (Transformation|SetActorLocation "-500.000000, 0, 0" false false)
  (Variables|Default|SetAttach_To_Objs (Utilities|Array|MakeArray "ObjectTypeQuery1" "ObjectTypeQuery2" "ObjectTypeQuery4"))
  (Variables|Default|SetMin_Max_Num_Def_Tree "(X=40.000000,Y=80.000000)")
  (Variables|Default|SetMin_Max_Num_Def_Grass "(X=50.000000,Y=100.000000)")
  (Variables|Default|SetMin_Max_Num_Def_Rocks "(X=30.000000,Y=50.000000)")
  (CallFunction|FMakeInstMeshArrays)
  (Utilities|FlowControl|Delay 5.0)
  (Utilities|Time|SetTimerbyEvent (delegate Custom|Remove_Instance_Timer) 1.0 true))

(fn ConstructionScript)

(fn FMakeInstMeshArrays
  (for _index (range 0 (- (Utilities|Array|Length (Variables|Meshes|GetTree_Arr)) 1))
    (bind _returnvalue (AddComponent|AddInstancedStaticMeshComponent false))
    (Utilities|Array|Add (Variables|Default|GetInst_Mesh_Tree_Arr) _returnvalue))
  (for _index_2 (range 0 (- (Utilities|Array|Length (Variables|Meshes|GetGrass_Arr)) 1))
    (bind _returnvalue_2 (AddComponent|AddInstancedStaticMeshComponent false))
    (Utilities|Array|Add (Variables|Default|GetInst_Mesh_Grass_Arr) _returnvalue_2))
  (for _index_3 (range 0 (- (Utilities|Array|Length (Variables|Meshes|GetRocks_Arr)) 1))
    (bind _returnvalue_3 (AddComponent|AddInstancedStaticMeshComponent false))
    (Utilities|Array|Add (Variables|Default|GetInst_Mesh_Rocks_Arr) _returnvalue_3)))

(fn FSpawnFoliage
  (params (Min_Max_Num :type Vector%202D%20Structure) (Min_Max_Scale :type Vector%202D%20Structure) (Foliage_Block_Sphere :type Float%20%28single-precision%29) (Spawn_Loc :type Vector) (Inst_Mesh_Arr :type Array%20of%20Instanced%20Static%20Mesh%20Component%20Object%20References) (Static_Mesh_Arr :type Array%20of%20Static%20Mesh%20Object%20References))
  (LocalVariables|SetL_Min_Max_Num Min_Max_Num)
  (LocalVariables|SetL_Min_Max_Scale Min_Max_Scale)
  (LocalVariables|SetL_Block_Sphere Foliage_Block_Sphere)
  (LocalVariables|SetL_Spawn_Loc Spawn_Loc)
  (for _index (range 0 (- (Utilities|Array|Length Inst_Mesh_Arr) 1))
    (Components|StaticMesh|SetStaticMesh (Utilities|Array|Get(acopy) Inst_Mesh_Arr _index) (Utilities|Array|Get(acopy) Static_Mesh_Arr _index))
    ;[1 1 1] Set   Start / End   LineTrace
    (LocalVariables|SetL_Line_Trace_Start (Math|Vector|MakeVector (.x (Math|Random|RandomPointinBoundingBox (LocalVariables|GetL_Spawn_Loc) (.BoxExtent (Collision|GetComponentBounds (Variables|Default|GetContainer))))) (.y (Math|Random|RandomPointinBoundingBox (LocalVariables|GetL_Spawn_Loc) (.BoxExtent (Collision|GetComponentBounds (Variables|Default|GetContainer))))) (+ (.z (Math|Random|RandomPointinBoundingBox (LocalVariables|GetL_Spawn_Loc) (.BoxExtent (Collision|GetComponentBounds (Variables|Default|GetContainer))))) 5e+03)))
    (if (Utilities|Array|IsValidIndex (LocalVariables|GetL_Locations_Arr))
      (for _array_element (LocalVariables|GetL_Locations_Arr)
        (if (< (Math|Vector|Distance2D(Vector) (Math|Vector2D|MakeVector2D (.x (LocalVariables|GetL_Line_Trace_Start)) (.y (LocalVariables|GetL_Line_Trace_Start))) _array_element) (LocalVariables|GetL_Block_Sphere))
          (LocalVariables|SetL_Can_Add false)))
      (if (LocalVariables|GetL_Can_Add)
        (Utilities|Array|Add (LocalVariables|GetL_Locations_Arr) (Math|Vector2D|MakeVector2D (.x (LocalVariables|GetL_Line_Trace_Start)) (.y (LocalVariables|GetL_Line_Trace_Start))) :!label _label)
        (LocalVariables|SetL_Line_Trace_End (+ (LocalVariables|GetL_Line_Trace_Start) (* (* (Transformation|GetActorUpVector) -1) 5e+03)))
        (bind (_outhit _returnvalue) (Collision|LineTraceForObjects (LocalVariables|GetL_Line_Trace_Start) (LocalVariables|GetL_Line_Trace_End) (Variables|Default|GetAttach_To_Objs) true 0 "None" true "(R=1.000000,G=0.000000,B=0.000000,A=1.000000)" "(R=0.000000,G=1.000000,B=0.000000,A=1.000000)" 1.0))
        (if _returnvalue
          (bind _returnvalue_2 (Components|InstancedStaticMesh|AddInstance (Utilities|Array|Get(acopy) Inst_Mesh_Arr _index) (Math|Transform|MakeTransform (.ImpactPoint (Collision|BreakHitResult _outhit)) (Math|Rotator|MakeRotator 0.0 0.0 (Math|Random|RandomFloatinRange 0.0 3.6e+02)) (* "1.000000,1.000000,1.000000" (Math|Random|RandomFloatinRange (.x (LocalVariables|GetL_Min_Max_Scale)) (.y (LocalVariables|GetL_Min_Max_Scale)))))))
          (Development|PrintString (Utilities|String|ToString(Integer) _returnvalue_2)))
        (else
          (LocalVariables|SetL_Can_Add true)))
      (else
        (goto _label))))
  (Utilities|Array|Clear (LocalVariables|GetL_Locations_Arr))
  (LocalVariables|SetL_Can_Add true)
  (LocalVariables|SetL_Try_Num 0))

(fn FDestroyInstance
  (params (Array :type Array%20of%20Instanced%20Static%20Mesh%20Component%20Object%20References) (Destroy_Range_X :type Float%20%28single-precision%29))
  (LocalVariables|SetDestroy_Range Destroy_Range_X)
  (for _array_element Array
    (for _index (range 0 (- (Components|InstancedStaticMesh|GetInstanceCount _array_element) 1))
      (if (< (+ (.x (.location (.OutInstanceTransform (Components|InstancedStaticMesh|GetInstanceTransform _array_element _index false)))) (LocalVariables|GetDestroy_Range)) (Variables|Default|GetCurr_Pawn_Location_X))
        (Class|InstancedStaticMeshComponent|RemoveInstance _array_element _index)))))